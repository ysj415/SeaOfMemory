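; Story-driven ship actor that reacts when the player character reaches it or its locked box, based on the StorySubsystem's current line.
; ShipOverlap checks the overlapping actor and its attached actors for the character, fires a one-time arrival event during Ship Phone, and clears guide text on exit during Goto Ship.
; DoorOverlap shows Korean password-clue or interaction hints by story stage, clearing the quest at Goto Ship.
; Both volumes maintain overlap flags.
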(event `self.ShipOverlap.OnComponentBeginOverlap`
  (params (OverlappedComponent :type "PrimitiveComponent Object Reference") (OtherActor :type "Actor Object Reference") (OtherComp :type "PrimitiveComponent Object Reference") (OtherBodyIndex :type Integer) (bFromSweep :type Boolean) (SweepResult :type "HitResult Structure (by ref)"))
  (`|ExecutionSequence`
    (:`then_0`
      (for _array_element (`self.GetAttachedActors` OtherActor true false)
        (bind _asbp_sombase_character (cast `/Game/Blueprint/Character/BP_SOMBaseCharacter` _array_element))
        (set `self.IsShipOverlap` true)
        (switch `QuestLine` (`StorySubsystem.CurrentLine` (subsystem `StorySubsystem`))
          (:`ShipPhone`
            (`/Engine/EditorBlueprintResources/StandardMacros.DoOnce` false :!label _label
              (:`Completed`
                (bind _returnvalue (`GameplayStatics.GetActorOfClass` "/Script/Engine.LevelScriptActor"))
                (message `/Game/Blueprint/QuestInterfac.ArriveShip` _returnvalue)
                (`/Game/Blueprint/Character/BP_SOMBaseCharacter.ArriveShipevent` _asbp_sombase_character)))))))
    (:`then_1`
      (cast `/Game/Blueprint/Character/BP_SOMBaseCharacter` OtherActor)
      (set `self.IsShipOverlap` true)
      (switch `QuestLine` (`StorySubsystem.CurrentLine` (subsystem `StorySubsystem`))
        (:`ShipPhone`
          (goto _label))))))

(event `self.ShipOverlap.OnComponentEndOverlap`
  (params (OverlappedComponent :type "PrimitiveComponent Object Reference") (OtherActor :type "Actor Object Reference") (OtherComp :type "PrimitiveComponent Object Reference") (OtherBodyIndex :type Integer))
  (`|ExecutionSequence`
    (:`then_0`
      (for _array_element (`self.GetAttachedActors` OtherActor true false)
        (bind _asbp_sombase_character (cast `/Game/Blueprint/Character/BP_SOMBaseCharacter` _array_element))
        (set `self.IsShipOverlap` false)
        (switch `QuestLine` (`StorySubsystem.CurrentLine` (subsystem `StorySubsystem`))
          (:`GotoShip`
            (`/Game/Blueprint/Character/BP_SOMBaseCharacter.SetGuideLineOff` _asbp_sombase_character)))))
    (:`then_1`
      (bind _asbp_sombase_character_2 (cast `/Game/Blueprint/Character/BP_SOMBaseCharacter` OtherActor))
      (set `self.IsShipOverlap` false)
      (switch `QuestLine` (`StorySubsystem.CurrentLine` (subsystem `StorySubsystem`))
        (:`GotoShip`
          (`/Game/Blueprint/Character/BP_SOMBaseCharacter.SetGuideLineOff` _asbp_sombase_character_2))))))

(event `self.DoorOverlap.OnComponentBeginOverlap`
  (params (OverlappedComponent :type "PrimitiveComponent Object Reference") (OtherActor :type "Actor Object Reference") (OtherComp :type "PrimitiveComponent Object Reference") (OtherBodyIndex :type Integer) (bFromSweep :type Boolean) (SweepResult :type "HitResult Structure (by ref)"))
  (bind _asbp_sombase_character (cast `/Game/Blueprint/Character/BP_SOMBaseCharacter` OtherActor))
  (switch `QuestLine` (`StorySubsystem.CurrentLine` (subsystem `StorySubsystem`))
    (:`GotoShip`
      (`/Game/Blueprint/Character/BP_SOMBaseCharacter.SetGuideLineScript` _asbp_sombase_character true "상자가 잠겨 있다... 비밀번호가 될 만한 단서를 찾아보자.")
      (`StorySubsystem.ClearCurrentQuest` (subsystem `StorySubsystem`)))
    (:`Item`
      (`/Game/Blueprint/Character/BP_SOMBaseCharacter.SetGuideLineScript` _asbp_sombase_character true "상자가 잠겨 있다... 비밀번호가 될 만한 단서를 찾아보자."))
    (:`CompletetoGetItem`
      (`/Game/Blueprint/Character/BP_SOMBaseCharacter.SetGuideLineScript` _asbp_sombase_character true "'P'를 눌러 상자와 상호작용하기")))
  (set `self.IsDoorOverlap` true))

(event `self.DoorOverlap.OnComponentEndOverlap`
  (params (OverlappedComponent :type "PrimitiveComponent Object Reference") (OtherActor :type "Actor Object Reference") (OtherComp :type "PrimitiveComponent Object Reference") (OtherBodyIndex :type Integer))
  (bind _asbp_sombase_character (cast `/Game/Blueprint/Character/BP_SOMBaseCharacter` OtherActor))
  (set `self.IsDoorOverlap` false)
  (switch `QuestLine` (`StorySubsystem.CurrentLine` (subsystem `StorySubsystem`))
    (:`Item`
      _)
    (:`CompletetoGetItem`
      _))
  (`/Game/Blueprint/Character/BP_SOMBaseCharacter.SetGuideLineOff` _asbp_sombase_character))

(fn `UserConstructionScript`)