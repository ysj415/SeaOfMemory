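; Player boat actor with trigger zones for diving into the sea and climbing back aboard.
; Two dive boxes and two boarding boxes set readiness flags on BP_SOMBaseCharacter and toggle Korean key prompts; GetOnBoatOverlapBox1 shows its prompt on exit, opposite to the others.
; BeginPlay caches the player, engine, old car, ship and item actors.
; Tick mirrors the player's drive and on-boat state, which this graph never uses.
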(event `self.ReceiveBeginPlay`
  (bind _asbp_sombase_character (cast `/Game/Blueprint/Character/BP_SOMBaseCharacter` (`GameplayStatics.GetPlayerCharacter` 0)))
  (set `self.As BP SOMBase Character` _asbp_sombase_character)
  (bind _returnvalue (`GameplayStatics.GetActorOfClass` "/Game/Blueprint/Mesh/BP_Engine.BP_Engine_C"))
  (set `self.BP_Engine` _returnvalue)
  (bind _returnvalue_2 (`GameplayStatics.GetActorOfClass` "/Game/Blueprint/Mesh/BP_OldCar.BP_OldCar_C"))
  (set `self.BP_OldCar` _returnvalue_2)
  (bind _returnvalue_3 (`GameplayStatics.GetActorOfClass` "/Game/Blueprint/Mesh/BP_Ship.BP_Ship_C"))
  (set `self.BP_Ship` _returnvalue_3)
  (bind _returnvalue_4 (`GameplayStatics.GetActorOfClass` "/Game/Blueprint/Mesh/BP_Item.BP_Item_C"))
  (set `self.BP_Item` _returnvalue_4))

(event `self.ReceiveTick`
  (params (DeltaSeconds :type "Float (single-precision)"))
  (bind _as_bp_sombase_character (`self.As BP SOMBase Character`))
  (`/Engine/EditorBlueprintResources/StandardMacros.IsValid` _as_bp_sombase_character
    (:`Is Valid`
      (set `self.Drive Turn Time` (`/Game/Blueprint/Character/BP_SOMBaseCharacter.Drive Turn Time` _as_bp_sombase_character))
      (set `self.Drive Degree` (`/Game/Blueprint/Character/BP_SOMBaseCharacter.Drive Degree` _as_bp_sombase_character))
      (set `self.Is Drive` (`/Game/Blueprint/Character/BP_SOMBaseCharacter.Is Drive` _as_bp_sombase_character))
      (set `self.Is on Boat` (`/Game/Blueprint/Character/BP_SOMBaseCharacter.IsOnBoat` _as_bp_sombase_character)))))

(event `self.DiveOverlapBox1.OnComponentBeginOverlap`
  (params (OverlappedComponent :type "PrimitiveComponent Object Reference") (OtherActor :type "Actor Object Reference") (OtherComp :type "PrimitiveComponent Object Reference") (OtherBodyIndex :type Integer) (bFromSweep :type Boolean) (SweepResult :type "HitResult Structure (by ref)"))
  (bind _asbp_sombase_character (cast `/Game/Blueprint/Character/BP_SOMBaseCharacter` OtherActor))
  (set `SOMBaseCharacter.IsReadyToDiving` true _asbp_sombase_character)
  (`/Game/Blueprint/Character/BP_SOMBaseCharacter.SetGuideLineUpScript` _asbp_sombase_character true "'Space Bar'를 눌러 바다로 뛰어들기"))

(event `self.DiveOverlapBox1.OnComponentEndOverlap`
  (params (OverlappedComponent :type "PrimitiveComponent Object Reference") (OtherActor :type "Actor Object Reference") (OtherComp :type "PrimitiveComponent Object Reference") (OtherBodyIndex :type Integer))
  (bind _asbp_sombase_character (cast `/Game/Blueprint/Character/BP_SOMBaseCharacter` OtherActor))
  (set `SOMBaseCharacter.IsReadyToDiving` false _asbp_sombase_character)
  (`/Game/Blueprint/Character/BP_SOMBaseCharacter.SetGuideLineUpOff` _asbp_sombase_character))

(event `self.DiveOverlapBox2.OnComponentBeginOverlap`
  (params (OverlappedComponent :type "PrimitiveComponent Object Reference") (OtherActor :type "Actor Object Reference") (OtherComp :type "PrimitiveComponent Object Reference") (OtherBodyIndex :type Integer) (bFromSweep :type Boolean) (SweepResult :type "HitResult Structure (by ref)"))
  (bind _asbp_sombase_character (cast `/Game/Blueprint/Character/BP_SOMBaseCharacter` OtherActor))
  (set `SOMBaseCharacter.IsReadyToDiving` true _asbp_sombase_character)
  (`/Game/Blueprint/Character/BP_SOMBaseCharacter.SetGuideLineUpScript` _asbp_sombase_character true "'Space Bar'를 눌러 바다로 뛰어들기"))

(event `self.DiveOverlapBox2.OnComponentEndOverlap`
  (params (OverlappedComponent :type "PrimitiveComponent Object Reference") (OtherActor :type "Actor Object Reference") (OtherComp :type "PrimitiveComponent Object Reference") (OtherBodyIndex :type Integer))
  (bind _asbp_sombase_character (cast `/Game/Blueprint/Character/BP_SOMBaseCharacter` OtherActor))
  (set `SOMBaseCharacter.IsReadyToDiving` false _asbp_sombase_character)
  (`/Game/Blueprint/Character/BP_SOMBaseCharacter.SetGuideLineUpOff` _asbp_sombase_character))

(event `self.GetOnBoatOverlapBox2.OnComponentBeginOverlap`
  (params (OverlappedComponent :type "PrimitiveComponent Object Reference") (OtherActor :type "Actor Object Reference") (OtherComp :type "PrimitiveComponent Object Reference") (OtherBodyIndex :type Integer) (bFromSweep :type Boolean) (SweepResult :type "HitResult Structure (by ref)"))
  (bind _asbp_sombase_character (cast `/Game/Blueprint/Character/BP_SOMBaseCharacter` OtherActor))
  (set `SOMBaseCharacter.IsReadyToGetOnBoat` true _asbp_sombase_character)
  (`/Game/Blueprint/Character/BP_SOMBaseCharacter.SetGuideLineUpScript` _asbp_sombase_character true "'O'를 눌러 배로 돌아가기"))

(event `self.GetOnBoatOverlapBox2.OnComponentEndOverlap`
  (params (OverlappedComponent :type "PrimitiveComponent Object Reference") (OtherActor :type "Actor Object Reference") (OtherComp :type "PrimitiveComponent Object Reference") (OtherBodyIndex :type Integer))
  (bind _asbp_sombase_character (cast `/Game/Blueprint/Character/BP_SOMBaseCharacter` OtherActor))
  (set `SOMBaseCharacter.IsReadyToGetOnBoat` false _asbp_sombase_character)
  (`/Game/Blueprint/Character/BP_SOMBaseCharacter.SetGuideLineUpOff` _asbp_sombase_character))

(event `self.GetOnBoatOverlapBox1.OnComponentEndOverlap`
  (params (OverlappedComponent :type "PrimitiveComponent Object Reference") (OtherActor :type "Actor Object Reference") (OtherComp :type "PrimitiveComponent Object Reference") (OtherBodyIndex :type Integer))
  (bind _asbp_sombase_character (cast `/Game/Blueprint/Character/BP_SOMBaseCharacter` OtherActor))
  (set `SOMBaseCharacter.IsReadyToGetOnBoat` false _asbp_sombase_character)
  (`/Game/Blueprint/Character/BP_SOMBaseCharacter.SetGuideLineUpScript` _asbp_sombase_character true "'O'를 눌러 배로 돌아가기"))

(event `self.GetOnBoatOverlapBox1.OnComponentBeginOverlap`
  (params (OverlappedComponent :type "PrimitiveComponent Object Reference") (OtherActor :type "Actor Object Reference") (OtherComp :type "PrimitiveComponent Object Reference") (OtherBodyIndex :type Integer) (bFromSweep :type Boolean) (SweepResult :type "HitResult Structure (by ref)"))
  (bind _asbp_sombase_character (cast `/Game/Blueprint/Character/BP_SOMBaseCharacter` OtherActor))
  (set `SOMBaseCharacter.IsReadyToGetOnBoat` true _asbp_sombase_character)
  (`/Game/Blueprint/Character/BP_SOMBaseCharacter.SetGuideLineUpOff` _asbp_sombase_character))

(fn `UserConstructionScript`)