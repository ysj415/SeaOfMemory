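; BP_OldCar is an old car prop that serves as the boat-part pickup point during the Engine story step.
; Tick polls StorySubsystem's CurrentLine and activates EngineFX only on that step, switching it off on the other lines.
; Overlap during that step registers the car as the character's OvelapEngine and shows a Korean "press B" pickup prompt.
; Leaving the overlap clears both; the pickup itself is not handled here.
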(event `self.ReceiveTick`
  (params (DeltaSeconds :type "Float (single-precision)"))
  (bind _enginefx (`self.EngineFX`))
  (switch `QuestLine` (`StorySubsystem.CurrentLine` (subsystem `StorySubsystem`))
    (:`OpenPhone`
      (`ActorComponent.SetActive` _enginefx false false :!label _label))
    (:`DrivingBoat`
      (goto _label))
    (:`GotoUnderWater`
      (goto _label))
    (:`Engine`
      (`ActorComponent.SetActive` _enginefx true false))
    (:`GotoBoat`
      (goto _label))
    (:`ShipPhone`
      (goto _label))
    (:`GotoShip`
      (goto _label))
    (:`Item`
      (goto _label))
    (:`CompletetoGetItem`
      (goto _label))
    (:`Clear`
      (goto _label))))

(event `self.OldCarOverlap.OnComponentBeginOverlap`
  (params (OverlappedComponent :type "PrimitiveComponent Object Reference") (OtherActor :type "Actor Object Reference") (OtherComp :type "PrimitiveComponent Object Reference") (OtherBodyIndex :type Integer) (bFromSweep :type Boolean) (SweepResult :type "HitResult Structure (by ref)"))
  (bind _asbp_sombase_character (cast `/Game/Blueprint/Character/BP_SOMBaseCharacter` OtherActor))
  (switch `QuestLine` (`StorySubsystem.CurrentLine` (subsystem `StorySubsystem`))
    (:`Engine`
      (set `/Game/Blueprint/Character/BP_SOMBaseCharacter.OvelapEngine` self _asbp_sombase_character)
      (set `self.IsOldCarOverlap` true)
      (`/Game/Blueprint/Character/BP_SOMBaseCharacter.SetGuideLineScript` _asbp_sombase_character true "'B'를 눌러 배의 부품을 줍기"))))

(event `self.OldCarOverlap.OnComponentEndOverlap`
  (params (OverlappedComponent :type "PrimitiveComponent Object Reference") (OtherActor :type "Actor Object Reference") (OtherComp :type "PrimitiveComponent Object Reference") (OtherBodyIndex :type Integer))
  (bind _asbp_sombase_character (cast `/Game/Blueprint/Character/BP_SOMBaseCharacter` OtherActor))
  (set `/Game/Blueprint/Character/BP_SOMBaseCharacter.OvelapEngine` null _asbp_sombase_character)
  (set `self.IsOldCarOverlap` false)
  (`/Game/Blueprint/Character/BP_SOMBaseCharacter.SetGuideLineScript` _asbp_sombase_character false ""))

(fn `UserConstructionScript`)