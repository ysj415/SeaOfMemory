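; Story-driven item pickup actor, a box whose hints and Niagara highlight follow the StorySubsystem's current story line.
; Tick switches the Niagara effect on only during the Item line and off for the other handled lines.
; Overlap by a BP_SOMBaseCharacter shows a Korean guide line chosen by story line, flagging IsItemOverlap during Goto Ship and Item.
; Leaving the overlap clears the flag and guide line.
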(event `self.ReceiveTick`
  (params (DeltaSeconds :type "Float (single-precision)"))
  (bind _niagara (`self.Niagara`))
  (switch `QuestLine` (`StorySubsystem.CurrentLine` (subsystem `StorySubsystem`))
    (:`OpenPhone`
      (`ActorComponent.SetActive` _niagara false false :!label _label))
    (:`DrivingBoat`
      (goto _label))
    (:`GotoUnderWater`
      (goto _label))
    (:`Engine`
      (goto _label))
    (:`GotoBoat`
      (goto _label))
    (:`ShipPhone`
      (goto _label))
    (:`GotoShip`
      (goto _label))
    (:`Item`
      (`ActorComponent.SetActive` _niagara true false))
    (:`CompletetoGetItem`
      (goto _label))
    (:`Clear`
      (goto _label))))

(event `self.ItemOverlap.OnComponentBeginOverlap`
  (params (OverlappedComponent :type "PrimitiveComponent Object Reference") (OtherActor :type "Actor Object Reference") (OtherComp :type "PrimitiveComponent Object Reference") (OtherBodyIndex :type Integer) (bFromSweep :type Boolean) (SweepResult :type "HitResult Structure (by ref)"))
  (bind _asbp_sombase_character (cast `/Game/Blueprint/Character/BP_SOMBaseCharacter` OtherActor))
  (switch `QuestLine` (`StorySubsystem.CurrentLine` (subsystem `StorySubsystem`))
    (:`Engine`
      (`/Game/Blueprint/Character/BP_SOMBaseCharacter.SetGuideLineScript` _asbp_sombase_character true "먼저 부품을 찾고 오자"))
    (:`GotoBoat`
      (`/Game/Blueprint/Character/BP_SOMBaseCharacter.SetGuideLineScript` _asbp_sombase_character true "우선 보트로 돌아가자."))
    (:`GotoShip`
      (set `self.IsItemOverlap` true :!label _label_2)
      (`/Game/Blueprint/Character/BP_SOMBaseCharacter.SetGuideLineScript` _asbp_sombase_character true "상자 안에 뭔가 있다. 확인해 보자."))
    (:`Item`
      (goto _label_2))))

(event `self.ItemOverlap.OnComponentEndOverlap`
  (params (OverlappedComponent :type "PrimitiveComponent Object Reference") (OtherActor :type "Actor Object Reference") (OtherComp :type "PrimitiveComponent Object Reference") (OtherBodyIndex :type Integer))
  (bind _asbp_sombase_character (cast `/Game/Blueprint/Character/BP_SOMBaseCharacter` OtherActor))
  (set `self.IsItemOverlap` false)
  (`/Game/Blueprint/Character/BP_SOMBaseCharacter.SetGuideLineOff` _asbp_sombase_character))

(fn `UserConstructionScript`)