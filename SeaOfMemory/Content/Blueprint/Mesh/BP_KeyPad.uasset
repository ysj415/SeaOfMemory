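; Interactive keypad that registers itself with the player character on overlap and asks for a passcode.
; Interacting turns off its Niagara effect, blends to the keypad camera, enables mouse clicks and links the child-actor BP_KeyButtons back to itself.
; Button input edits the text display, and confirming compares it to KeyPadCode with sound and color feedback.
; A correct code restores the player view and destroys the keypad, while a wrong one resets entry after a delay.
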(event `self.Box.OnComponentBeginOverlap`
  (params (OverlappedComponent :type "PrimitiveComponent Object Reference") (OtherActor :type "Actor Object Reference") (OtherComp :type "PrimitiveComponent Object Reference") (OtherBodyIndex :type Integer) (bFromSweep :type Boolean) (SweepResult :type "HitResult Structure (by ref)"))
  (if (== OtherActor (`GameplayStatics.GetPlayerPawn` 0))
    (bind _asbp_sombase_character (cast `/Game/Blueprint/Character/BP_SOMBaseCharacter` OtherActor))
    (set `/Game/Blueprint/Character/BP_SOMBaseCharacter.KeyInteractActor` self _asbp_sombase_character)
    (set `self.As BP SOMBase Character` _asbp_sombase_character)))

(event `self.Box.OnComponentEndOverlap`
  (params (OverlappedComponent :type "PrimitiveComponent Object Reference") (OtherActor :type "Actor Object Reference") (OtherComp :type "PrimitiveComponent Object Reference") (OtherBodyIndex :type Integer))
  (if (== OtherActor (`GameplayStatics.GetPlayerPawn` 0))
    (bind _asbp_sombase_character (cast `/Game/Blueprint/Character/BP_SOMBaseCharacter` OtherActor))
    (set `/Game/Blueprint/Character/BP_SOMBaseCharacter.KeyInteractActor` null _asbp_sombase_character)
    (set `self.As BP SOMBase Character` null)))

(event `On Interact`
  (bind _returnvalue (`GameplayStatics.GetPlayerController` 0))
  (bind _entercode (`self.EnterCode`))
  (`self.Turn on Niagara` false)
  (set `self.IsInteraction` true)
  (`PlayerController.SetViewTargetWithBlend` (`GameplayStatics.GetPlayerController` 0) (`ActorComponent.GetOwner` (`self.Camera`)) 0.4 "VTBlend_Linear" 0.0 false)
  (set `PlayerController.bShowMouseCursor` true _returnvalue :!label _label)
  (set `PlayerController.bEnableClickEvents` true _returnvalue)
  (set `PlayerController.bEnableMouseOverEvents` true _returnvalue)
  (`TextRenderComponent.K2_SetText` _entercode "")
  (`TextRenderComponent.SetTextRenderColor` _entercode (make `Color` 1 1 1 255))
  (bind _output_get (set `self.ButtonArray` (`|MakeArray` (`self.1`) (`self.2`) (`self.3`) (`self.4`) (`self.5`) (`self.6`) (`self.7`) (`self.8`) (`self.9`) (`self.0`) (`self.back`) (`self.enter`))))
  (for _array_element _output_get
    (bind _asbp_key_buttons (cast `/Game/Blueprint/Mesh/BP_KeyButtons` (`ChildActorComponent.ChildActor` _array_element)))
    (set `/Game/Blueprint/Mesh/BP_KeyButtons.KeyPadActor` self _asbp_key_buttons)))

(event `Initiate`
  (goto _label))

(event `ButtonEnter`
  (params (Value :type Text) (Confirm :type Boolean) (Backspace :type Boolean))
  (bind _entercode (`self.EnterCode`))
  (if Confirm
    (`self.Confirmed`)
    (elif Backspace
      (`self.Backspace`)
      (elif (`self.CanEnter`)
        (`GameplayStatics.PlaySound2D` "/Engine/VREditor/Sounds/UI/Click_on_Button.Click_on_Button" 1.0 1.0 0.0 null null)
        (`TextRenderComponent.K2_SetText` _entercode (`KismetTextLibrary.Conv_StringToText` (`KismetStringLibrary.Replace` (`KismetTextLibrary.Conv_TextToString` (`TextRenderComponent.Text` (`self.EnterCode`))) (`KismetStringLibrary.GetSubstring` "...." 0 (`KismetStringLibrary.Len` (`self.KeyPadCode`))))))
        (`TextRenderComponent.K2_SetText` _entercode (`KismetTextLibrary.Conv_StringToText` (`KismetStringLibrary.Concat_StrStr` (`KismetTextLibrary.Conv_TextToString` (`TextRenderComponent.Text` (`self.EnterCode`))) (`KismetTextLibrary.Conv_TextToString` Value))))
        (`TextRenderComponent.SetTextRenderColor` (`self.EnterCode`) (make `Color` 200 200 200 255))))))

(event `Backspace`
  (bind _entercode (`self.EnterCode`))
  (bind _returnvalue (`KismetTextLibrary.Conv_TextToString` (`TextRenderComponent.Text` _entercode)))
  (`TextRenderComponent.K2_SetText` _entercode (`KismetTextLibrary.Conv_StringToText` (`KismetStringLibrary.GetSubstring` _returnvalue 0 (- (`KismetStringLibrary.Len` _returnvalue) 1)))))

(event `Confirmed`
  (bind _returnvalue (`GameplayStatics.GetPlayerController` 0))
  (bind _returnvalue_2 (`GameplayStatics.GetPlayerController` 0))
  (bind _entercode (`self.EnterCode`))
  (bind _entercode_2 (`self.EnterCode`))
  (if (`KismetStringLibrary.EqualEqual_StrStr` (`self.KeyPadCode`) (`KismetTextLibrary.Conv_TextToString` (`TextRenderComponent.Text` (`self.EnterCode`))))
    (`|ExecutionSequence`
      (:`then_0`
        (`TextRenderComponent.K2_SetText` _entercode_2 "Correct  Passcode")
        (`TextRenderComponent.SetTextRenderColor` _entercode_2 (make `Color` 0 255 0 255))
        (`KismetSystemLibrary.Delay` 1.0)
        (set `PlayerController.bShowMouseCursor` false _returnvalue_2)
        (set `PlayerController.bEnableClickEvents` false _returnvalue_2)
        (set `PlayerController.bEnableMouseOverEvents` false _returnvalue_2)
        (for _array_element (`self.ButtonArray`)
          (cast `/Game/Blueprint/Mesh/BP_KeyButtons` (`ChildActorComponent.ChildActor` _array_element)))
        (`PlayerController.SetViewTargetWithBlend` (`GameplayStatics.GetPlayerController` 0) (`ActorComponent.GetOwner` (`SOMBaseCharacter.Camera` (cast `/Game/Blueprint/Character/BP_SOMBaseCharacter` (`GameplayStatics.GetPlayerPawn` 0) :!pure true))) 0.4 "VTBlend_Linear" 0.0 false)
        (`/Game/Blueprint/Character/BP_SOMBaseCharacter.ClearKeypad` (`self.As BP SOMBase Character`))
        (`self.K2_DestroyActor`))
      (:`then_1`
        (set `self.CanEnter` false)
        (`GameplayStatics.PlaySound2D` "/Engine/EditorSounds/Notifications/CompileSuccess.CompileSuccess" 1.0 1.0 0.0 null null)))
    (else
      (`|ExecutionSequence`
        (:`then_0`
          (`TextRenderComponent.K2_SetText` _entercode "Wrong  Passcode")
          (`TextRenderComponent.SetTextRenderColor` _entercode (make `Color` 0 0 255 255))
          (set `PlayerController.bEnableClickEvents` false _returnvalue)
          (set `PlayerController.bEnableMouseOverEvents` false _returnvalue)
          (`KismetSystemLibrary.Delay` 1.0)
          (for _array_element_2 (`self.ButtonArray`)
            (cast `/Game/Blueprint/Mesh/BP_KeyButtons` (`ChildActorComponent.ChildActor` _array_element_2)))
          (`self.Initiate`)
          (set `self.CanEnter` true))
        (:`then_1`
          (set `self.CanEnter` false)
          (`GameplayStatics.PlaySound2D` "/Engine/EditorSounds/Notifications/CompileFailed.CompileFailed" 1.0 1.0 0.0 null null))))))

(fn `Turn on Niagara`
  (params (NewParam :type Boolean))
  (bind _niagara (`self.niagara`))
  (`/Engine/EditorBlueprintResources/StandardMacros.IsValid` _niagara
    (:`Is Valid`
      (`ActorComponent.SetActive` (`/Game/Blueprint/Mesh/BP_BoxTrap.Niagara` _niagara) NewParam false))))

(fn `UserConstructionScript`)